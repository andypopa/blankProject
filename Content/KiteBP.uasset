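; Kite actor that the player can reposition and rotate with the mouse.
; A left click on the mesh or its rotation handle starts moving or rotating, and the next click ends it.
; Tick snaps the actor to a line trace from the deprojected cursor while moving, or derives yaw from cursor offset since the click while rotating.
; When idle, hovering over the actor shows the handle and point light.
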(event EventBeginPlay)

(event Collision|EventActorBeginOverlap
  (params (OtherActor :type Actor%20Object%20Reference)))

(event EventTick
  (params (DeltaSeconds :type Float%20%28single-precision%29))
  (bind _returnvalue (Game|GetPlayerController 0))
  (bind _returnvalue_2 (Game|GetPlayerController 0))
  (bind _rotationstart (Variables|Default|GetRotationStart))
  (bind _worldlocation (Game|Player|ConvertMouseLocationToWorldSpace _returnvalue))
  (bind (_worldlocation_2 _worlddirection) (Game|Player|ConvertMouseLocationToWorldSpace _returnvalue_2))
  (bind _returnvalue_3 (- _rotationstart _worldlocation))
  (bind (_x _y) (Math|Vector|BreakVector _returnvalue_3))
  (if (Variables|Default|GetMoving)
    (bind _outhit (Collision|LineTraceByChannel _worldlocation_2 (+ (* _worlddirection 2e+03) _worlddirection) "TraceTypeQuery1" false 0 "None"))
    (Transformation|SetActorLocation (.Location (Collision|BreakHitResult _outhit)) false false)
    (elif (Variables|Default|GetRotating)
      (Transformation|SetActorRotation (Math|Rotator|MakeRotator 0.0 0.0 (* (+ _x _y) 25.0)))
      (elif (== (.HitActor (Collision|BreakHitResult (.HitResult (Game|Player|GetHitResultUnderCursorbyChannel (Game|GetPlayerController 0) "TraceTypeQuery1" true)))) self)
        (Rendering|SetVisibility (Variables|Default|GetRotationHandle) true false)
        (Rendering|SetVisibility (Variables|Default|GetPointLight) true false)
        (else
          (Rendering|SetVisibility (Variables|Default|GetRotationHandle) false false)
          (Rendering|SetVisibility (Variables|Default|GetPointLight) false false))))))

(event Input|MouseEvents|LeftMouseButton
  (params (Key :type Key%20Structure :default "AnyKey"))
  (bind _returnvalue (Game|GetPlayerController 0))
  (bind _hitresult (Game|Player|GetHitResultUnderCursorbyChannel _returnvalue "TraceTypeQuery1" true))
  (bind _hitcomponent (Collision|BreakHitResult _hitresult))
  (:Pressed
    (if (Variables|Default|GetMoving)
      (Variables|Default|SetMoving false)
      (elif (Variables|Default|GetRotating)
        (Variables|Default|SetRotating false)
        (elif (== (Variables|Default|GetStaticMesh) _hitcomponent)
          (Variables|Default|SetMoving true)
          (elif (== _hitcomponent (Variables|Default|GetRotationHandle))
            (Variables|Default|SetRotating true)
            (Variables|Default|SetRotationStart (.WorldLocation (Game|Player|ConvertMouseLocationToWorldSpace (Game|GetPlayerController 0))))))))))

(fn ConstructionScript)